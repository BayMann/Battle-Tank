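; BP_Tank is the player-controlled tank Blueprint, and its graph handles only camera orbit and zoom.
; Turn and LookUp axis input add local yaw to YawRoot and pitch to PitchRoot, scaled by a fixed factor with no delta time or pitch limit.
; Zoom and Unzoom presses step PitchRoot's arm length in or out, bounded by minimum and maximum distance checks.
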(event `InputAxis|Turn`
  (params (AxisValue :type "Float (single-precision)"))
  (`SceneComponent.K2_AddLocalRotation` (`self.YawRoot`) (`KismetMathLibrary.MakeRotator` 0.0 0.0 (* AxisValue 5.0)) false false))

(event `InputAxis|LookUp`
  (params (AxisValue :type "Float (single-precision)"))
  (`SceneComponent.K2_AddLocalRotation` (`self.PitchRoot`) (`KismetMathLibrary.MakeRotator` 0.0 (* AxisValue 5.0)) false false))

(event `InputAction|Zoom`
  (params (Key :type "Key Structure"))
  (bind _pitchroot (`self.PitchRoot`))
  (bind _targetarmlength (`SpringArmComponent.TargetArmLength` _pitchroot))
  (:`Pressed`
    (if (<= _targetarmlength 200.0)
      (set `SpringArmComponent.TargetArmLength` 200.0 _pitchroot)
      (else
        (set `SpringArmComponent.TargetArmLength` (- _targetarmlength 100.0) _pitchroot)))))

(event `InputAction|Unzoom`
  (params (Key :type "Key Structure"))
  (bind _pitchroot (`self.PitchRoot`))
  (bind _targetarmlength (`SpringArmComponent.TargetArmLength` _pitchroot))
  (:`Pressed`
    (if (>= _targetarmlength 1000.0)
      (set `SpringArmComponent.TargetArmLength` 1000.0 _pitchroot)
      (else
        (set `SpringArmComponent.TargetArmLength` (+ _targetarmlength 100.0) _pitchroot)))))

(fn `UserConstructionScript`)